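; Manager actor for a card-ordering puzzle that the player solves while focused on an inspectable object.
; It binds to every BP_Card's click event, and each pair of clicked cards swaps places with an eased move.
; Pressing F while focused checks that Card1 to Card4 ascend along X.
; Success stops the timer, returns view and movement to the player and destroys the inspect actor; failure flags a ten-second timer penalty.
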(event `self.ReceiveBeginPlay`
  (`|ExecutionSequence`
    (:`then_0`
      (`self.EnableInput` (`GameplayStatics.GetPlayerController` 0)))
    (:`then_1`
      (bind _outactors (`GameplayStatics.GetAllActorsOfClass` "/Game/BP_Card.BP_Card_C"))
      (for _array_element _outactors
        (add `/Game/BP_Card.CardClicked` _array_element (`|CreateDelegate` :!event `OnCardClicked`))))))

(event `OnCardClicked`
  (params (ClickedCard :type "/Game/BP_Card Object Reference"))
  (bind _output (`|GetArrayItem` (`self.SelectedCard`) 1))
  (bind _output_2 (`|GetArrayItem` (`self.SelectedCard`)))
  (`KismetArrayLibrary.Array_Add` (`self.SelectedCard`) ClickedCard)
  (if (== (`KismetArrayLibrary.Array_Length` (`self.SelectedCard`)) 2)
    (bind _output_get (set `self.TempLocationA` (`self.K2_GetActorLocation` _output_2)))
    (bind _output_get_2 (set `self.TempLocationB` (`self.K2_GetActorLocation` _output)))
    (`KismetSystemLibrary.MoveComponentTo` (`Actor.RootComponent` _output_2) _output_get_2 (struct :`Yaw` 90.0) true true 0.25)
    (`KismetSystemLibrary.MoveComponentTo` (`Actor.RootComponent` _output) _output_get (struct :`Yaw` 90.0) true true 0.25)
    (`KismetArrayLibrary.Array_Clear` (`self.SelectedCard`))))

(event `Key|F`
  (params (Key :type "Key Structure"))
  (bind _x (.x (`self.K2_GetActorLocation` (`self.Card3`))))
  (bind _x_2 (.x (`self.K2_GetActorLocation` (`self.Card2`))))
  (:`Pressed`
    (if (`/Game/BP_Cards.isFocused?` (`self.Inspect`))
      (if (and (< (.x (`self.K2_GetActorLocation` (`self.Card1`))) _x_2) (< _x_2 _x) (< _x (.x (`self.K2_GetActorLocation` (`self.Card4`)))))
        (`/Engine/EditorBlueprintResources/StandardMacros.DoOnce` false
          (:`Completed`
            (set `/Game/BP_Cards.Success` true (`self.Inspect`))
            (bind _aswbp_timer (cast `/Game/WBP_Timer` (`WidgetComponent.GetUserWidgetObject` (`/Game/BP_TV.ScreenTimerWidget` (`self.TimeRef`)))))
            (`KismetSystemLibrary.K2_ClearTimer` _aswbp_timer "TickTimer")
            (set `PlayerController.bShowMouseCursor` false (`GameplayStatics.GetPlayerController` 0))
            (`PlayerController.SetViewTargetWithBlend` (`GameplayStatics.GetPlayerController` 0) (`/Game/BP_Cards.PlayerRef` (`self.Inspect`)) 0.3 "VTBlend_Linear" 0.0 false)
            (`Widget.SetVisibility` (`/Game/FirstPerson/Widgets/WBP_HUD.CrosshairBorder` (`/Game/FirstPerson/Blueprints/BP_FirstPersonCharacter.HUDRef` (`/Game/BP_Cards.PlayerRef` (`self.Inspect`)))) "Visible")
            (`CharacterMovementComponent.SetMovementMode` (`Character.CharacterMovement` (`/Game/BP_Cards.PlayerRef` (`self.Inspect`))) "MOVE_Walking" 0)
            (`WidgetBlueprintLibrary.SetInputMode_GameOnly` (`GameplayStatics.GetPlayerController` 0))
            (`KismetSystemLibrary.Delay` 0.3)
            (`self.K2_DestroyActor` (`self.Inspect`))))
        (else
          (bind _aswbp_timer_2 (cast `/Game/WBP_Timer` (`WidgetComponent.GetUserWidgetObject` (`/Game/BP_TV.ScreenTimerWidget` (`self.TimeRef`)))))
          (set `/Game/WBP_Timer.Subtruct10Seconds` true _aswbp_timer_2))))))

(fn `UserConstructionScript`)