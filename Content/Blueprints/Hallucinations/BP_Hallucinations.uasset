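; Trigger-box hallucination sequence that activates only once the electrical panel puzzle is solved.
; On overlap, timelines chained from each other's Update pins drive blur, vignette, effect weight and inscription glow through MPC_Hallucinations, alongside raised post-process bloom.
; After delays, it hides the door, disables its collision and reveals steam.
; Leaving reverses effect weight and glow, lowers bloom and restores the door, but leaves steam visible.
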(event `self.ReceiveBeginPlay`
  ; Event Begin Play
  (`|ExecutionSequence`
    (:`then_0`
      (bind _asbp_first_person_character (cast `/Game/FirstPerson/Blueprints/BP_FirstPersonCharacter` (`GameplayStatics.GetPlayerCharacter` 0)))
      (set `self.PlayerRef` _asbp_first_person_character)
      (bind _outactors (`GameplayStatics.GetAllActorsOfClass` "/Game/Blueprints/ElectricPanel/BP_ElectricalPanel.BP_ElectricalPanel_C"))
      (set `self.ElectricalPanelRef` (`|GetArrayItem` _outactors))
      (`self.SetActorHiddenInGame` (`self.SteamRef`) true))
    (:`then_1`
      (bind _outactors_2 (`GameplayStatics.GetAllActorsOfClass` "/Script/Engine.PostProcessVolume"))
      (bind _output_get (set `self.PostProcessOrigin` (`|GetArrayItem` _outactors_2)))
      (bind _output_get_2 (set `self.PostProcess` _output_get))
      (set `PostProcessVolume.Settings` (`PostProcessVolume.Settings` _output_get_2) _output_get_2))))

(event `self.BoxTrigger.OnComponentBeginOverlap`
  (params (OverlappedComponent :type "PrimitiveComponent Object Reference") (OtherActor :type "Actor Object Reference") (OtherComp :type "PrimitiveComponent Object Reference") (OtherBodyIndex :type Integer) (bFromSweep :type Boolean) (SweepResult :type "HitResult Structure (by ref)"))
  (bind _doorref (`self.DoorRef`))
  (bind ((`AutoExposureMinBrightness` _autoexposureminbrightness) (`AutoExposureMaxBrightness` _autoexposuremaxbrightness) (`WeightedBlendables` _weightedblendables)) (break `PostProcessSettings` (`PostProcessVolume.Settings` (`self.PostProcess`))))
  (if (`/Game/Blueprints/ElectricPanel/BP_ElectricalPanel.PuzzleSolved?` (`self.ElectricalPanelRef`))
    (bind (_direction _blurweight) (`Timeline|BlurWeight`)
      (:`Update`
        (`KismetMaterialLibrary.SetScalarParameterValue` "/Game/Graphics/MPC_Hallucinations.MPC_Hallucinations" "BlurWeight" _blurweight)
        (bind (_direction_2 _vignetteintensityweight) (`Timeline|VignetteIntensityWeight`)
          (:`Update`
            (`KismetMaterialLibrary.SetScalarParameterValue` "/Game/Graphics/MPC_Hallucinations.MPC_Hallucinations" "VignetteIntensity" _vignetteintensityweight)
            (bind (_direction_3 _vignettezoomweight) (`Timeline|VignetteZoomWeight`)
              (:`Update`
                (`KismetMaterialLibrary.SetScalarParameterValue` "/Game/Graphics/MPC_Hallucinations.MPC_Hallucinations" "VignetteZoom" _vignettezoomweight)
                (bind (_direction_4 _blurweight_2) (`Timeline|BlurWeightDecline`)
                  (:`Update`
                    (`KismetMaterialLibrary.SetScalarParameterValue` "/Game/Graphics/MPC_Hallucinations.MPC_Hallucinations" "BlurWeight" _blurweight_2)
                    (`|ExecutionSequence`
                      (:`then_0`
                        (`KismetSystemLibrary.Delay` 2.5)
                        (bind (_direction_5 _weight) (`Timeline|EffectWieght`)
                          (:`Update`
                            (`KismetMaterialLibrary.SetScalarParameterValue` "/Game/Graphics/MPC_Hallucinations.MPC_Hallucinations" "EffectWeight" _weight)
                            (bind _output_get (set `self.BloomIntensity` 4.0))
                            (set `PostProcessVolume.Settings` (make `PostProcessSettings` :`BloomIntensity` _output_get :`AutoExposureMinBrightness` _autoexposureminbrightness :`AutoExposureMaxBrightness` _autoexposuremaxbrightness :`WeightedBlendables` _weightedblendables) (`self.PostProcess`))
                            (bind (_direction_6 _intensity) (`Timeline|Timeline_1`)
                              (:`Update`
                                (`KismetMaterialLibrary.SetScalarParameterValue` "/Game/Graphics/MPC_Hallucinations.MPC_Hallucinations" "InscriptionsEmissionIntensity" _intensity))))))
                      (:`then_1`
                        (`KismetSystemLibrary.Delay` 2.0)
                        (`SceneComponent.SetVisibility` (`Actor.RootComponent` _doorref) false false)
                        (`PrimitiveComponent.SetCollisionEnabled` (`StaticMeshActor.StaticMeshComponent` _doorref) "NoCollision")
                        (`self.SetActorHiddenInGame` (`self.SteamRef`) false)))))))))))))

(event `self.BoxTrigger.OnComponentEndOverlap`
  (params (OverlappedComponent :type "PrimitiveComponent Object Reference") (OtherActor :type "Actor Object Reference") (OtherComp :type "PrimitiveComponent Object Reference") (OtherBodyIndex :type Integer))
  (bind _doorref (`self.DoorRef`))
  (bind ((`AutoExposureMinBrightness` _autoexposureminbrightness) (`AutoExposureMaxBrightness` _autoexposuremaxbrightness) (`WeightedBlendables` _weightedblendables)) (break `PostProcessSettings` (`PostProcessVolume.Settings` (`self.PostProcess`))))
  (if (`/Game/Blueprints/ElectricPanel/BP_ElectricalPanel.PuzzleSolved?` (`self.ElectricalPanelRef`))
    (bind (_direction _weight) (`Timeline|EffectWieghtReverse`)
      (:`Update`
        (`KismetMaterialLibrary.SetScalarParameterValue` "/Game/Graphics/MPC_Hallucinations.MPC_Hallucinations" "EffectWeight" _weight)
        (bind (_direction_2 _intensity) (`Timeline|Timeline_2`)
          (:`Update`
            (`KismetMaterialLibrary.SetScalarParameterValue` "/Game/Graphics/MPC_Hallucinations.MPC_Hallucinations" "InscriptionsEmissionIntensity" _intensity)
            (bind _output_get (set `self.BloomIntensity` 0.675))
            (set `PostProcessVolume.Settings` (make `PostProcessSettings` :`BloomIntensity` (`KismetMathLibrary.FInterpTo` 4.0 _output_get 2.0 0.1) :`AutoExposureMinBrightness` _autoexposureminbrightness :`AutoExposureMaxBrightness` _autoexposuremaxbrightness :`WeightedBlendables` _weightedblendables) (`self.PostProcess`))
            (`KismetSystemLibrary.Delay` 1.0)
            (`SceneComponent.SetVisibility` (`Actor.RootComponent` _doorref) true false)
            (`PrimitiveComponent.SetCollisionEnabled` (`StaticMeshActor.StaticMeshComponent` _doorref) "QueryAndPhysics")))))))

(fn `UserConstructionScript`)