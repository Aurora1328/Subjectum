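; Keycard door that swings open on interact when its door type is Locked Door and CanOpen is true.
; At BeginPlay it binds to every BP_Keycard's collected event to set HasKey, though Interact never reads that flag directly.
; With UseDOT off, a DoOnce-guarded timeline rotates the hinge's yaw with a sound and marks the door open, with no closing path.
; Failed attempts play a locked-door sound.
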(event `self.ReceiveBeginPlay`
  (bind _outactors (`GameplayStatics.GetAllActorsOfClass` "/Game/Blueprints/LabDoor/BP_Keycard.BP_Keycard_C"))
  (for _array_element _outactors
    (bind _asbp_keycard (cast `/Game/Blueprints/LabDoor/BP_Keycard` _array_element))
    (add `/Game/Blueprints/LabDoor/BP_Keycard.OnKeyCollected` _asbp_keycard (delegate `KeyCollected`))))

(event `KeyCollected`
  (set `self.HasKey` true))

(event `self.Interact`
  (params (Character :type "/Game/FirstPerson/Blueprints/BP_FirstPersonCharacter Object Reference"))
  (switch `/Game/Blueprints/Enums/E_DoorType` (`.DoorType_7_BEEF82C24F50735CB94DE59FC6BB5F8C` (break `/Game/Blueprints/Structs/S_DoorInfo` (`.DoorInfo_22_379011D0461B9A6CF354F4BF657FFEFC` (break `/Game/Blueprints/Structs/S_ItemInfo` (`self.ItemInfo`)))))
    (:`NewEnumerator2`
      (if (`self.CanOpen`)
        (if (`self.UseDOT?`) :!label _label
          _
          (elif (not (`self.DoorOpen?`))
            (`/Engine/EditorBlueprintResources/StandardMacros.DoOnce` false :!label _label_2
              (:`Completed`
                (`GameplayStatics.PlaySound2D` "/Game/Audio/Sounds/door_open-1.door_open-1" 1.0 1.0 0.0 null null)
                (bind (_direction _doorangle) (`Timeline|DoorOpen` :!via `PlayFromStart`)
                  (:`Update`
                    (`SceneComponent.K2_SetRelativeRotation` (`self.Hinge`) (`KismetMathLibrary.MakeRotator` 0.0 0.0 _doorangle) false false))
                  (:`Finished`
                    (set `self.DoorOpen?` true)
                    (goto _label_2 :!via `Reset`)))))))
        (else
          (`GameplayStatics.PlaySound2D` "/Game/Audio/Sounds/door_closed_try.door_closed_try" 1.0 1.0 0.0 null null)
          (if (not true)
            (goto _label)))))))

(fn `UserConstructionScript`
  (`parent.UserConstructionScript`))