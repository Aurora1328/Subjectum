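; BP_Switch is an interactable light switch that toggles a referenced rect light between a configurable intensity and zero.
; Interact checks the actor from the SphereTrigger overlap against the player character, then plays a click, flips IsLightOn and prints the state.
; Inner and outer collision spheres swap near and far interaction icons as overlaps begin and end.
; The construction script sizes all three spheres from radius variables.
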(event `self.SphereTrigger.OnComponentBeginOverlap`
  (params (OverlappedComponent :type "PrimitiveComponent Object Reference") (OtherActor :type "Actor Object Reference") (OtherComp :type "PrimitiveComponent Object Reference") (OtherBodyIndex :type Integer) (bFromSweep :type Boolean) (SweepResult :type "HitResult Structure (by ref)")))

(event `/Game/Blueprints/BPI_Interact.Interact`
  (bind _rectlightcomponent (`RectLight.RectLightComponent` (`self.light`)))
  (if (== (stale `self.SphereTrigger.OnComponentBeginOverlap` OtherActor) (`GameplayStatics.GetPlayerCharacter` 0))
    (`GameplayStatics.PlaySound2D` "/Engine/VREditor/Sounds/UI/Click_on_Button.Click_on_Button" 1.0 1.0 0.0 null null)
    (if (not (`self.isLightOn`))
      (set `self.isLightOn` true)
      (`KismetSystemLibrary.PrintString` "LightOn")
      (`LightComponent.SetIntensity` _rectlightcomponent (`self.LightIntensity`))
      (else
        (set `self.isLightOn` false)
        (`KismetSystemLibrary.PrintString` "LightOff")
        (`LightComponent.SetIntensity` _rectlightcomponent 0.0)))))

(event `self.InnerSphereCollision.OnComponentBeginOverlap`
  (params (OverlappedComponent :type "PrimitiveComponent Object Reference") (OtherActor :type "Actor Object Reference") (OtherComp :type "PrimitiveComponent Object Reference") (OtherBodyIndex :type Integer) (bFromSweep :type Boolean) (SweepResult :type "HitResult Structure (by ref)"))
  (`SceneComponent.SetVisibility` (`self.InnerInteractIcon`) true false)
  (`SceneComponent.SetVisibility` (`self.OuterInteractIcon`) false false))

(event `self.InnerSphereCollision.OnComponentEndOverlap`
  (params (OverlappedComponent :type "PrimitiveComponent Object Reference") (OtherActor :type "Actor Object Reference") (OtherComp :type "PrimitiveComponent Object Reference") (OtherBodyIndex :type Integer))
  (`SceneComponent.SetVisibility` (`self.InnerInteractIcon`) false false)
  (`SceneComponent.SetVisibility` (`self.OuterInteractIcon`) true false))

(event `self.OuterSphereCollision.OnComponentBeginOverlap`
  (params (OverlappedComponent :type "PrimitiveComponent Object Reference") (OtherActor :type "Actor Object Reference") (OtherComp :type "PrimitiveComponent Object Reference") (OtherBodyIndex :type Integer) (bFromSweep :type Boolean) (SweepResult :type "HitResult Structure (by ref)"))
  (`SceneComponent.SetVisibility` (`self.OuterInteractIcon`) true false))

(event `self.OuterSphereCollision.OnComponentEndOverlap`
  (params (OverlappedComponent :type "PrimitiveComponent Object Reference") (OtherActor :type "Actor Object Reference") (OtherComp :type "PrimitiveComponent Object Reference") (OtherBodyIndex :type Integer))
  (`SceneComponent.SetVisibility` (`self.OuterInteractIcon`) false false))

(fn `UserConstructionScript`
  (`SphereComponent.SetSphereRadius` (`self.InnerSphereCollision`) (`self.Inner Sphere Radius`) true)
  (`SphereComponent.SetSphereRadius` (`self.OuterSphereCollision`) (`self.Outer Sphere Radius`) true)
  (`SphereComponent.SetSphereRadius` (`self.SphereTrigger`) (`self.SphereTriggerRadius`) true))