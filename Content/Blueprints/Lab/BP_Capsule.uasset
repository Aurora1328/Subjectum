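; Lab capsule actor with a couch mesh and hinged door, exposing events to lower, raise, open, close and fast-close it.
; Timelines add height offsets to the saved actor location and roll offsets to the saved DoorRoot rotation.
; Lowering also sets KeycardInteract after a delay triggered from the timeline update.
; Each motion plays its own sound, attached to the couch except fast close, which plays at world origin.
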(event `DownCapsule`
  (`GameplayStatics.SpawnSoundAttached` "/Game/Audio/Sound_new/capsule_down-1.capsule_down-1" (`self.CouchMesh`) "None" (0.0 0.0 0.0) (struct) "KeepRelativeOffset" false 1.0 1.0 0.0 "/Game/Audio/CapsuleAttenuation.CapsuleAttenuation" null)
  (set `self.StartLocation` (`self.K2_GetActorLocation`))
  (bind (_direction _heightoffset) (`Timeline|MoveDownTimeline` :!via `PlayFromStart`)
    (:`Update`
      (`self.K2_SetActorLocation` (`KismetMathLibrary.MakeVector` (.x (`self.StartLocation`)) (.y (`self.StartLocation`)) (+ _heightoffset (.z (`self.StartLocation`)))))
      (`KismetSystemLibrary.Delay` 4.0)
      (set `self.KeycardInteract?` true))))

(event `UpCapsule`
  (`GameplayStatics.SpawnSoundAttached` "/Game/Audio/Sound_new/capsule_up.capsule_up" (`self.CouchMesh`) "None" (0.0 0.0 0.0) (struct) "KeepRelativeOffset" false 1.0 1.0 0.0 "/Game/Audio/CapsuleAttenuation.CapsuleAttenuation" null)
  (set `self.StartLocation` (`self.K2_GetActorLocation`))
  (bind (_direction _heightoffset) (`Timeline|MoveUpTimeline` :!via `PlayFromStart`)
    (:`Update`
      (`self.K2_SetActorLocation` (`KismetMathLibrary.MakeVector` (.x (`self.StartLocation`)) (.y (`self.StartLocation`)) (+ _heightoffset (.z (`self.StartLocation`)))))
      (`KismetSystemLibrary.Delay` 4.0))))

(event `OpenDoor`
  (`GameplayStatics.SpawnSoundAttached` "/Game/Audio/Sound_new/capsule_open.capsule_open" (`self.CouchMesh`) "None" (0.0 0.0 0.0) (struct) "KeepRelativeOffset" false 1.0 1.0 0.0 "/Game/Audio/CapsuleAttenuation.CapsuleAttenuation" null)
  (set `self.StartRotationDoor` (.rotation (`SceneComponent.GetRelativeTransform` (`self.DoorRoot`))))
  (bind (_direction _heightoffset) (`Timeline|OpenTimeline` :!via `PlayFromStart`)
    (:`Update`
      (`SceneComponent.K2_SetRelativeRotation` (`self.DoorRoot`) (`KismetMathLibrary.MakeRotator` (+ (.roll (`self.StartRotationDoor`)) _heightoffset) (.pitch (`self.StartRotationDoor`)) (.yaw (`self.StartRotationDoor`))) false false))))

(event `CloseDoor`
  (`GameplayStatics.SpawnSoundAttached` "/Game/Audio/Sound_new/capsule_close.capsule_close" (`self.CouchMesh`) "None" (0.0 0.0 0.0) (struct) "KeepRelativeOffset" false 1.0 1.0 0.0 "/Game/Audio/CapsuleAttenuation.CapsuleAttenuation" null)
  (set `self.StartRotationDoor` (.rotation (`SceneComponent.GetRelativeTransform` (`self.DoorRoot`))))
  (bind (_direction _heightoffset) (`Timeline|CloseTimeline` :!via `PlayFromStart`)
    (:`Update`
      (`SceneComponent.K2_SetRelativeRotation` (`self.DoorRoot`) (`KismetMathLibrary.MakeRotator` (+ (.roll (`self.StartRotationDoor`)) _heightoffset) (.pitch (`self.StartRotationDoor`)) (.yaw (`self.StartRotationDoor`))) false false))))

(event `CloseDoorFast`
  (`GameplayStatics.PlaySoundAtLocation` "/Game/Audio/capsule_close_fast.capsule_close_fast" (0.0 0.0 0.0) (struct) 0.5 1.0 0.0 null null null null)
  (set `self.StartRotationDoor` (.rotation (`SceneComponent.GetRelativeTransform` (`self.DoorRoot`))))
  (bind (_direction _heightoffset) (`Timeline|Timeline` :!via `PlayFromStart`)
    (:`Update`
      (`SceneComponent.K2_SetRelativeRotation` (`self.DoorRoot`) (`KismetMathLibrary.MakeRotator` (+ (.roll (`self.StartRotationDoor`)) _heightoffset) (.pitch (`self.StartRotationDoor`)) (.yaw (`self.StartRotationDoor`))) false false))))

(fn `UserConstructionScript`)