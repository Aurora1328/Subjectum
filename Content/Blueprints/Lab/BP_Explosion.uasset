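; BP_Explosion is a lab actor that holds six particle system components for explosion effects.
; Each component has its own TriggerExplosion function that activates it without a reset, so callers can fire each one separately.
; The event graph and construction script are empty, so nothing in the Blueprint itself triggers the effects.
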(fn `TriggerExplosion`
  (`ActorComponent.Activate` (`self.ParticleSystem`) false))

(fn `TriggerExplosion1`
  (`ActorComponent.Activate` (`self.ParticleSystem1`) false))

(fn `TriggerExplosion2`
  (`ActorComponent.Activate` (`self.ParticleSystem2`) false))

(fn `TriggerExplosion3`
  (`ActorComponent.Activate` (`self.ParticleSystem3`) false))

(fn `TriggerExplosion4`
  (`ActorComponent.Activate` (`self.ParticleSystem4`) false))

(fn `TriggerExplosion5`
  (`ActorComponent.Activate` (`self.ParticleSystem5`) false))

(fn `UserConstructionScript`)