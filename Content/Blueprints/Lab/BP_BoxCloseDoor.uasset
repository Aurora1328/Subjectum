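; BP_BoxCloseDoor is a one-shot trigger that plays a scripted door-slam and explosion sequence when BP_FirstPersonCharacter enters its box.
; The overlap passes a DoOnce, then calls CloseDoorFast on every BP_Capsule.
; Delays chained from that loop lead to the Birthday sound, then TriggerExplosion on every BP_Explosion, adding a WBP_BlackScreen widget to the viewport for each.
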(event `self.Box.OnComponentBeginOverlap`
  (params (OverlappedComponent :type "PrimitiveComponent Object Reference") (OtherActor :type "Actor Object Reference") (OtherComp :type "PrimitiveComponent Object Reference") (OtherBodyIndex :type Integer) (bFromSweep :type Boolean) (SweepResult :type "HitResult Structure (by ref)"))
  (cast `/Game/FirstPerson/Blueprints/BP_FirstPersonCharacter` OtherActor)
  (`/Engine/EditorBlueprintResources/StandardMacros.DoOnce` false
    (:`Completed`
      (bind _outactors (`GameplayStatics.GetAllActorsOfClass` "/Game/Blueprints/Lab/BP_Capsule.BP_Capsule_C"))
      (for _array_element _outactors
        (`/Game/Blueprints/Lab/BP_Capsule.CloseDoorFast` _array_element)
        (`KismetSystemLibrary.Delay` 1.5)
        (`GameplayStatics.PlaySound2D` "/Game/Audio/Sounds/Birthday.Birthday" 1.0 1.0 0.0 null null)
        (`KismetSystemLibrary.Delay` 5.0)
        (bind _outactors_2 (`GameplayStatics.GetAllActorsOfClass` "/Game/Blueprints/Lab/BP_Explosion.BP_Explosion_C"))
        (for _array_element_2 _outactors_2
          (`/Game/Blueprints/Lab/BP_Explosion.TriggerExplosion` _array_element_2)
          (bind _returnvalue (`|CreateWidget` "/Game/UI/PC/WBP_BlackScreen.WBP_BlackScreen_C"))
          (`UserWidget.AddToViewport` _returnvalue 0))))))

(fn `UserConstructionScript`)