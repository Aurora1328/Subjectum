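; Locked bedroom door for the children's room that swings open on its hinge via timelines once unlocked.
; Two near-duplicate interact events spend held keys (one key or all) when no ID is required, then open the door unless UseDOT is set.
; An UnlockDoor binding made at BeginPlay also unlocks it when this door is the target.
; CloseDoor swings it shut after a short delay, with DoOnce gates limiting replays.
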(event `self.ReceiveBeginPlay`
  (set `self.HasPlayedSound` false)
  (`parent.ReceiveBeginPlay`)
  (`self.UnlockDoorEvent`))

(event `self.Interact`
  (params (Character :type "/Game/FirstPerson/Blueprints/BP_FirstPersonCharacter Object Reference"))
  (bind _playerref (`self.PlayerRef`))
  (switch `/Game/Blueprints/Enums/E_DoorType` (`.DoorType_7_BEEF82C24F50735CB94DE59FC6BB5F8C` (break `/Game/Blueprints/Structs/S_DoorInfo` (`.DoorInfo_22_379011D0461B9A6CF354F4BF657FFEFC` (break `/Game/Blueprints/Structs/S_ItemInfo` (`self.ItemInfo`)))))
    (:`NewEnumerator2`
      (if (`self.DoorUnlocked?`)
        (if (not (`self.UseDOT?`)) :!label _label
          (bind _output_get (set `self.CanInteract` true))
          (if (not (and _output_get (`self.DoorOpen?`)))
            (`/Engine/EditorBlueprintResources/StandardMacros.DoOnce` false
              (:`Completed`
                (`GameplayStatics.PlaySound2D` "/Game/Audio/Sounds/door_open-1.door_open-1" 1.0 1.0 0.0 null null)
                (bind (_direction _doorangle) (`Timeline|Timeline_0` :!via `PlayFromStart`)
                  (:`Update`
                    (`SceneComponent.K2_SetRelativeRotation` (`self.Hinge`) (`KismetMathLibrary.MakeRotator` 0.0 0.0 _doorangle) false false))
                  (:`Finished`
                    (set `self.DoorOpen?` true)))))))
        (else
          (`GameplayStatics.PlaySound2D` "/Game/Audio/Sounds/door_closed_try.door_closed_try" 1.0 1.0 0.0 null null)
          (if (`self.IsIDRequired?`)
            _
            (elif (> (`/Game/FirstPerson/Blueprints/BP_FirstPersonCharacter.KeysHeld` (`self.PlayerRef`)) 0)
              (set `/Game/FirstPerson/Blueprints/BP_FirstPersonCharacter.KeysHeld` (`KismetMathLibrary.Clamp` (- (`/Game/FirstPerson/Blueprints/BP_FirstPersonCharacter.KeysHeld` _playerref) 1) 0 99) _playerref)
              (`/Game/FirstPerson/Blueprints/BP_FirstPersonCharacter.UpdateKeysHeld` (`self.PlayerRef`))
              (set `self.DoorUnlocked?` true)
              (goto _label))))))))

(event `EventInteract`
  (switch `/Game/Blueprints/Enums/E_DoorType` (`.DoorType_7_BEEF82C24F50735CB94DE59FC6BB5F8C` (break `/Game/Blueprints/Structs/S_DoorInfo` (`.DoorInfo_22_379011D0461B9A6CF354F4BF657FFEFC` (break `/Game/Blueprints/Structs/S_ItemInfo` (`self.ItemInfo`)))))
    (:`NewEnumerator2`
      (if (`self.DoorUnlocked?`)
        (if (not (`self.UseDOT?`)) :!label _label_2
          (bind _output_get (set `self.CanInteract` true))
          (if (not (and _output_get (`self.DoorOpen?`)))
            (`/Engine/EditorBlueprintResources/StandardMacros.DoOnce` false
              (:`Completed`
                (`GameplayStatics.PlaySound2D` "/Game/Audio/Sounds/door_open-1.door_open-1" 0.5 1.0 0.0 null null)
                (bind (_direction _doorangle) (`Timeline|Timeline_1` :!via `PlayFromStart`)
                  (:`Update`
                    (`SceneComponent.K2_SetRelativeRotation` (`self.Hinge`) (`KismetMathLibrary.MakeRotator` 0.0 0.0 _doorangle) false false))
                  (:`Finished`
                    (set `self.DoorOpen?` true)))))))
        (else
          (`GameplayStatics.PlaySound2D` "/Game/Audio/Sounds/door_closed_try.door_closed_try" 1.0 1.0 0.0 null null)
          (if (`self.IsIDRequired?`)
            _
            (elif (> (`/Game/FirstPerson/Blueprints/BP_FirstPersonCharacter.KeysHeld` (`self.PlayerRef`)) 0)
              (set `/Game/FirstPerson/Blueprints/BP_FirstPersonCharacter.KeysHeld` 0 (`self.PlayerRef`))
              (`/Game/FirstPerson/Blueprints/BP_FirstPersonCharacter.UpdateKeysHeld` (`self.PlayerRef`))
              (set `self.DoorUnlocked?` true)
              (goto _label_2))))))))

(event `CloseDoor`
  (bind _output_get (set `self.CanInteract` false))
  (`/Engine/EditorBlueprintResources/StandardMacros.DoOnce` _output_get
    (:`Completed`
      (`KismetSystemLibrary.Delay` 0.5)
      (`GameplayStatics.PlaySound2D` "/Game/Audio/Sounds/door_open-1.door_open-1" 0.5 1.0 0.0 null null)
      (bind (_direction _doorangle) (`Timeline|Timeline` :!via `PlayFromStart`)
        (:`Update`
          (`SceneComponent.K2_SetRelativeRotation` (`self.Hinge`) (`KismetMathLibrary.MakeRotator` 0.0 0.0 _doorangle) false false))
        (:`Finished`
          (set `self.DoorOpen?` false))))))

(event `UnlockDoorEvent`
  (add `self.UnlockDoor` (delegate `UnlockDoorBind`)))

(event `UnlockDoorBind` :!signature `self.UnlockDoor`
  (params (DoorToUnlock :type "Actor Object Reference"))
  (if (== DoorToUnlock self)
    (set `self.DoorUnlocked?` true)))

(fn `UserConstructionScript`
  (`parent.UserConstructionScript`))