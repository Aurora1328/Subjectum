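; BP_Item is an item actor that shows interaction icons as something comes within range.
; Overlapping the outer sphere shows an outer icon; overlapping the inner sphere swaps it for an inner icon, and each end overlap reverses the change.
; The overlap events do not filter which actor triggered them.
; The construction script applies the configurable radii to both spheres and assigns the static mesh.
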(event `self.InnerSphereCollision.OnComponentBeginOverlap`
  (params (OverlappedComponent :type "PrimitiveComponent Object Reference") (OtherActor :type "Actor Object Reference") (OtherComp :type "PrimitiveComponent Object Reference") (OtherBodyIndex :type Integer) (bFromSweep :type Boolean) (SweepResult :type "HitResult Structure (by ref)"))
  (`SceneComponent.SetVisibility` (`self.InnerInteractIcon`) true false)
  (`SceneComponent.SetVisibility` (`self.OuterInteractIcon`) false false))

(event `self.InnerSphereCollision.OnComponentEndOverlap`
  (params (OverlappedComponent :type "PrimitiveComponent Object Reference") (OtherActor :type "Actor Object Reference") (OtherComp :type "PrimitiveComponent Object Reference") (OtherBodyIndex :type Integer))
  (`SceneComponent.SetVisibility` (`self.InnerInteractIcon`) false false)
  (`SceneComponent.SetVisibility` (`self.OuterInteractIcon`) true false))

(event `self.OuterSphereCollision.OnComponentBeginOverlap`
  (params (OverlappedComponent :type "PrimitiveComponent Object Reference") (OtherActor :type "Actor Object Reference") (OtherComp :type "PrimitiveComponent Object Reference") (OtherBodyIndex :type Integer) (bFromSweep :type Boolean) (SweepResult :type "HitResult Structure (by ref)"))
  (`SceneComponent.SetVisibility` (`self.OuterInteractIcon`) true false))

(event `self.OuterSphereCollision.OnComponentEndOverlap`
  (params (OverlappedComponent :type "PrimitiveComponent Object Reference") (OtherActor :type "Actor Object Reference") (OtherComp :type "PrimitiveComponent Object Reference") (OtherBodyIndex :type Integer))
  (`SceneComponent.SetVisibility` (`self.OuterInteractIcon`) false false))

(fn `UserConstructionScript`
  (`SphereComponent.SetSphereRadius` (`self.InnerSphereCollision`) (`self.InnerSphereRadius`) true)
  (`SphereComponent.SetSphereRadius` (`self.OuterSphereCollision`) (`self.OuterSphereRadius`) true)
  (`StaticMeshComponent.SetStaticMesh` (`self.MeshComponent`) (`self.StaticMesh`)))